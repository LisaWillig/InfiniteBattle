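; AI controller for guard NPCs that runs the GuardBehaviour behavior tree and tracks who the guard currently senses.
; On BeginPlay it initializes the blackboard and starts the tree.
; AIPerception updates feed UpdateEnemyKey, which sets the Enemy blackboard key when an actor is sensed and clears it when sensing fails.
; Actors tagged Guard are ignored, so guards do not register each other as enemies.
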(event OnTargetPerceptionUpdated(AIPerception)
  (params (Actor :type Actor%20Object%20Reference) (Stimulus :type AI%20Stimulus%20Structure))
  (CallFunction|UpdateEnemyKey Actor Actor Stimulus))

(event EventBeginPlay
  (bind _blackboardcomponent (Class|AIController|UseBlackboard "/Game/AI/BehaviourTree/Blackboard.Blackboard"))
  (Variables|Default|SetBlackboardComp _blackboardcomponent)
  (AI|RunBehaviorTree "/Game/AI/BehaviourTree/GuardBehaviour.GuardBehaviour"))

(fn ConstructionScript)

(fn UpdateEnemyKey
  (params (ObjectValue :type Object%20Object%20Reference) (self2 :type Actor%20Object%20Reference) (AIStimulus :type AI%20Stimulus%20Structure%20%28by%20ref%29))
  (bind _returnvalue (Utilities|String|StringToName "Enemy"))
  (bind _blackboardcomp (Variables|Default|GetBlackboardComp))
  (if (not (Actor|ActorHasTag self2 "Guard"))
    (if (.bSuccessfullySensed (Utilities|Struct|BreakAIStimulus AIStimulus))
      (AI|Components|Blackboard|SetValueasObject _blackboardcomp _returnvalue ObjectValue)
      (else
        (AI|Components|Blackboard|ClearValue _blackboardcomp _returnvalue)))))