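; One tile of the infinite terrain level, which scatters rocks and spawns the game mode's count of AI enemies on BeginPlay.
; While the player is inside LockingArea, the barrier turns green and lets pawns overlap; leaving turns it red and scores once.
; The Garbage trigger asks the game mode for a new tile, then destroys this one with its attached actors and their guns.
; An Arrow component supplies the attach transform, and Tick keeps background music looping.
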(event OnComponentBeginOverlap(Garbage)
  (params (OverlappedComponent :type Primitive%20Component%20Object%20Reference) (OtherActor :type Actor%20Object%20Reference) (OtherComp :type Primitive%20Component%20Object%20Reference) (OtherBodyIndex :type Integer) (bFromSweep :type Boolean) (SweepResult :type Hit%20Result%20Structure%20%28by%20ref%29))
  (Utilities|IsPlayer OtherActor)
  (bind _asbp_infinite_terrain_game_mode (Utilities|Casting|CastToBP_InfiniteTerrainGameMode (Game|GetGameMode)))
  (Default|SpawnTile _asbp_infinite_terrain_game_mode)
  (CallFunction|DeleteLevel))

(event OnComponentEndOverlap(LockingArea)
  (params (OverlappedComponent :type Primitive%20Component%20Object%20Reference) (OtherActor :type Actor%20Object%20Reference) (OtherComp :type Primitive%20Component%20Object%20Reference) (OtherBodyIndex :type Integer))
  (Utilities|IsPlayer OtherActor)
  (CallFunction|Lock)
  (Utilities|FlowControl|DoOnce false
    (:Completed
      (bind _asbp_infinite_terrain_game_mode (Utilities|Casting|CastToBP_InfiniteTerrainGameMode (Game|GetGameMode)))
      (Default|IncreaseScore _asbp_infinite_terrain_game_mode))))

(event EventBeginPlay
  (CallFunction|Lock)
  (CallFunction|SpawnAI)
  (Class|Tile|PlaceActors "/Game/Levels/Probs/Rock2.Rock2_C" 0 5 0.1 0.8)
  (Class|Tile|PlaceActors "/Game/Levels/Probs/Rock1.Rock1_C" 5 10 0.2 5.0))

(event EventTick
  (params (DeltaSeconds :type Float%20%28single-precision%29))
  (CallFunction|BackgroundMusicLoop)
  (CallFunction|UnlockNextTile))

(fn ConstructionScript)

(fn GetAttachLocation
  (return (Transformation|GetWorldTransform (Variables|Default|GetArrow))))

(fn Unlock
  (bind _barrierwall (Variables|Default|GetBarrierWall))
  (Collision|SetCollisionEnabled _barrierwall "QueryAndPhysics")
  (Collision|SetCollisionResponsetoChannel _barrierwall "ECC_Pawn" "ECR_Overlap")
  (Collision|SetCollisionResponsetoChannel _barrierwall "ECC_GameTraceChannel3" "ECR_Block")
  (Rendering|Material|SetMaterial _barrierwall 0 "/Game/Levels/Terrain/MI_EmissiveBarrier_Green.MI_EmissiveBarrier_Green"))

(fn Lock
  (Collision|SetCollisionEnabled (Variables|Default|GetBarrierWall) "QueryAndPhysics")
  (Rendering|Material|SetMaterial (Variables|Default|GetBarrierWall) 0 "/Game/Levels/Terrain/MI_Barrier_Red.MI_Barrier_Red"))

(fn SpawnAI
  (bind _asbp_infinite_terrain_game_mode (Utilities|Casting|CastToBP_InfiniteTerrainGameMode (Game|GetGameMode)))
  (bind _enemynumber (Default|GetEnemyNumber _asbp_infinite_terrain_game_mode))
  (Class|Tile|PlaceAIPawns "/Game/Character/BP_Character.BP_Character_C" _enemynumber))

(fn BackgroundMusicLoop
  (if (not (Audio|Components|Audio|IsPlaying (Variables|Default|GetBackground)))
    (Audio|Components|Audio|Play (Variables|Default|GetBackground) 0.0)))

(fn UnlockNextTile
  (if (Collision|IsOverlappingActor (Variables|Default|GetLockingArea) (Game|GetPlayerCharacter 0) :!class /Script/Engine.PrimitiveComponent)
    (CallFunction|Unlock)))

(fn DeleteLevel
  (bind _arrayelement (Utilities|Array|ReverseforEachLoop (Actor|GetAttachedActors true))
    (:LoopBody
      (CallFunction|DeleteGun _arrayelement)
      (Actor|DestroyActor _arrayelement))
    (:Completed
      (Actor|DestroyActor))))

(fn DeleteGun
  (params (self2 :type Actor%20Object%20Reference))
  (bind _arrayelement (Utilities|Array|ReverseforEachLoop (Actor|GetAttachedActors self2 true))
    (:LoopBody
      (Utilities|IsValid _arrayelement
        (:Is%20Valid
          (bind _asbp_gun (Utilities|Casting|CastToBP_Gun _arrayelement))
          (Class|Gun|Delete _asbp_gun))))))