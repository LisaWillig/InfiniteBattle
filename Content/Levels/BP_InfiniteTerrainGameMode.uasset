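; Game mode for an endless tile-based level that tracks score, enemy count and the saved highscore.
; On start it chains four tiles by attach point, passing each a NavMeshBoundsVolume pool, and attaches a tutorial wall to the first.
; Tick watches for an invalid player character, then once saves through the GameInstance, shows a win screen for a beaten highscore or a death screen otherwise, and removes the HUD.
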(event Custom|StartGame
  (CallFunction|SetInitialHighscore)
  (Class|InfiniteTerrainGameMode|PopulateBoundsVolumePool)
  (for _index (range 0 3)
    (bind _newparam (CallFunction|SpawnTile))
    (CallFunction|SpawnTutorialWall (== _index 0) _newparam)))

(event EventTick
  (params (DeltaSeconds :type Float%20%28single-precision%29))
  (bind _returnvalue (Game|GetPlayerController 0))
  (Utilities|IsValid (Game|GetPlayerCharacter 0)
    (:Is%20Not%20Valid
      (Utilities|FlowControl|DoOnce false
        (:Completed
          (CallFunction|SaveHighscore)
          (if (Variables|Default|GetWin)
            (bind _returnvalue_2 (Game|ConstructObjectfromClass "/Game/UI/WBP_WinScreen.WBP_WinScreen_C" _returnvalue))
            (UserInterface|Viewport|AddtoViewport _returnvalue_2 0)
            (else
              (bind _returnvalue_3 (Game|ConstructObjectfromClass "/Game/UI/WBP_DeathScreen.WBP_DeathScreen_C" _returnvalue))
              (UserInterface|Viewport|AddtoViewport _returnvalue_3 0)))
          (bind _asbp_hud (Utilities|Casting|CastToBP_HUD (HUD|GetHUD _returnvalue)))
          (Default|RemoveHUD _asbp_hud))))))

(fn ConstructionScript)

(fn SpawnTile
  (Variables|Default|SetEnemyNumber (+ (Variables|Default|GetEnemyNumber) 1))
  (bind _returnvalue (Game|SpawnActorfromClass "/Game/Levels/Terrain/BP_Tile.BP_Tile_C" (Variables|Default|GetTransform) "Undefined" 0 0))
  (Class|Tile|SetPool _returnvalue (Variables|Default|GetNavMeshBoundsVolumePool))
  (bind _attach_transform (Default|GetAttachLocation _returnvalue))
  (Variables|Default|SetTransform _attach_transform)
  (return _returnvalue))

(fn IncreaseScore
  (bind _result (Math|Integer|IncrementInt (Variables|Default|GetScore))
    (:%20%20
      (Variables|Default|SetScore _result))))

(fn GetEnemyNumber
  (return (Variables|Default|GetEnemyNumber)))

(fn SpawnTutorialWall
  (params (Condition :type Boolean) (ParentActor :type Actor%20Object%20Reference))
  (if Condition
    (bind _returnvalue (Game|SpawnActorfromClass "/Game/Levels/Terrain/TutorialWall.TutorialWall_C" (Variables|Default|GetTutorial_Transform) "AlwaysSpawn" 0 0))
    (Transformation|AttachActorToActor _returnvalue ParentActor "None" "KeepRelative" "KeepRelative" "KeepRelative" true)))

(fn GetScore
  (return (Variables|Default|GetScore)))

(fn SaveHighscore
  (bind _score (Variables|Default|GetScore))
  (bind _asbp_game_instance (Utilities|Casting|CastToBP_GameInstance (Game|GetGameInstance)))
  (if (< (Variables|Default|GetHighscore) _score)
    (Variables|Default|SetWin true)
    (Variables|/Script/ReloadedBattle.SaveData|SetHighscore (Variables|/Game/Levels/BP_GameInstance.BP_GameInstance_C|GetSaveGameData _asbp_game_instance) _score))
  (SaveGame|SaveGametoSlot (Variables|/Game/Levels/BP_GameInstance.BP_GameInstance_C|GetSaveGameData _asbp_game_instance) (Variables|/Game/Levels/BP_GameInstance.BP_GameInstance_C|GetSaveSlots _asbp_game_instance)))

(fn SetInitialHighscore
  (bind _asbp_game_instance (Utilities|Casting|CastToBP_GameInstance (Game|GetGameInstance)))
  (Variables|Default|SetHighscore (Variables|/Game/Levels/BP_GameInstance.BP_GameInstance_C|GetHighscore _asbp_game_instance)))